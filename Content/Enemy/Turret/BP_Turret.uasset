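; BP_Turret is an enemy turret that tracks and shoots at the player while they are inside its Box trigger.
; Overlap by Bp_PlayerChar starts two looping timers by function name, and end overlap clears both.
; The fast timer turns Pivot toward player character 0 using a look-at from the actor's location.
; The slower timer spawns a BP_Turret_Projectile at the ProjectileSpawn transform.
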(event OnComponentBeginOverlap(Box)
  (params (OverlappedComponent :type Primitive%20Component%20Object%20Reference) (OtherActor :type Actor%20Object%20Reference) (OtherComp :type Primitive%20Component%20Object%20Reference) (OtherBodyIndex :type Integer) (bFromSweep :type Boolean) (SweepResult :type Hit%20Result%20Structure%20%28by%20ref%29))
  (Utilities|Casting|CastToBp_PlayerChar OtherActor)
  (Utilities|Time|SetTimerbyFunctionName 0 "FollowPlayer" 0.02 true)
  (Utilities|Time|SetTimerbyFunctionName 0 "fireAtPlayer" 1.0 true))

(event OnComponentEndOverlap(Box)
  (params (OverlappedComponent :type Primitive%20Component%20Object%20Reference) (OtherActor :type Actor%20Object%20Reference) (OtherComp :type Primitive%20Component%20Object%20Reference) (OtherBodyIndex :type Integer))
  (Utilities|Casting|CastToBp_PlayerChar OtherActor)
  (Utilities|Time|ClearTimerbyFunctionName 0 "FollowPlayer")
  (Utilities|Time|ClearTimerbyFunctionName 0 "fireAtPlayer"))

(event Custom|FollowPlayer
  (Transformation|SetWorldRotation (Variables|Default|GetPivot) (Math|Rotator|FindLookatRotation (Transformation|GetActorLocation) (Transformation|GetActorLocation (Game|GetPlayerCharacter 0))) false false))

(event Custom|fireAtPlayer
  (Game|SpawnActorfromClass "/Game/Enemy/Turret/BP_Turret_Projectile.BP_Turret_Projectile_C" (Transformation|GetWorldTransform (Variables|Default|GetProjectile%20Spawn)) "Undefined" "MultiplyWithRoot" 0 0))

(fn ConstructionScript)