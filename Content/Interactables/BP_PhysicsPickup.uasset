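; BP_PhysicsPickup is an interactable physics cube that the player can pick up and drop.
; INTInteract, if the player holds nothing, sets IsHolding, disables the cube's physics and collision, and snaps it to the player's Arrow1.
; INTDrop calls DetachFromActor and restores collision and physics, leaving IsHolding untouched.
; The construction script tints the cube through a dynamic material instance using PickupColor.
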(event EventINTInteract
  (params (PlayerRef :type Bp%20Player%20Char%20Object%20Reference))
  (bind _cube1 (Variables|Default|GetCube1))
  (if (not (Variables|/Game/Player/Bp_PlayerChar.Bp_PlayerChar_C|GetisHolding PlayerRef))
    (Variables|/Game/Player/Bp_PlayerChar.Bp_PlayerChar_C|SetisHolding PlayerRef true)
    (Physics|SetSimulatePhysics _cube1 false)
    (Collision|SetCollisionEnabled _cube1 "NoCollision")
    (Transformation|AttachComponentToComponent (Variables|Default|GetCube1) (Variables|/Game/Player/Bp_PlayerChar.Bp_PlayerChar_C|GetArrow1 PlayerRef) "None" "SnapToTarget" "KeepRelative" "KeepRelative" true)))

(event EventINTDrop
  (bind _cube1 (Variables|Default|GetCube1))
  (Transformation|DetachFromActor "KeepWorld" "KeepWorld" "KeepWorld")
  (Collision|SetCollisionEnabled _cube1 "QueryAndPhysics")
  (Physics|SetSimulatePhysics _cube1 true))

(fn ConstructionScript
  (bind _returnvalue (Rendering|Material|CreateDynamicMaterialInstance (Variables|Default|GetCube1) 0 "/Game/Interactables/AnimatedInteractables/Mat_Color.Mat_Color" "None" :!class /Script/Engine.PrimitiveComponent))
  (bind _output_get (Variables|Default|SetColorDMI _returnvalue))
  (Rendering|Material|SetVectorParameterValue _output_get "Color" (Variables|Default|GetPickupColor) :!class /Script/Engine.MaterialInstanceDynamic))