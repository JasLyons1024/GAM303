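; Interactable swinging door that opens when a player interacts with it, provided it is unlocked.
; A dot product of the actor's forward vector and the direction to the player picks which way it swings.
; A timeline lerps the yaw of Arrow1 to that angle, then reverses after a short delay to close it.
; The construction script tints the Cube with PickupColor through a dynamic material.
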(event Custom|ReverseTimeline
  (bind (_direction _alpha) (Timeline|Timeline Reverse)
    (:Update
      (Transformation|SetRelativeRotation (Variables|Default|GetArrow1) (Math|Rotator|MakeRotator 0.0 0.0 (Math|Float|Lerp 0.0 (stale EventINTInteract _returnvalue) _alpha)) false false))
    (:Finished
      (if (Utilities|Enum|Equal(Enum) _direction "Forward")
        (Utilities|FlowControl|Delay 5.0)
        (CallFunction|ReverseTimeline)))))

(event EventINTInteract
  (params (PlayerRef :type Bp%20Player%20Char%20Object%20Reference))
  (if (Variables|Default|GetisUnlocked)
    (bind _returnvalue (CallFunction|UpdateDoorAngle PlayerRef))
    (bind (_direction _alpha) (Timeline|Timeline Play)
      (:Update
        (Transformation|SetRelativeRotation (Variables|Default|GetArrow1) (Math|Rotator|MakeRotator 0.0 0.0 (Math|Float|Lerp 0.0 _returnvalue _alpha)) false false))
      (:Finished
        (if (Utilities|Enum|Equal(Enum) _direction "Forward")
          (Utilities|FlowControl|Delay 5.0)
          (CallFunction|ReverseTimeline))))))

(fn ConstructionScript
  (bind _returnvalue (Rendering|Material|CreateDynamicMaterialInstance (Variables|Default|GetCube) 0 "/Game/Interactables/AnimatedInteractables/Mat_Color.Mat_Color" "None" :!class /Script/Engine.PrimitiveComponent))
  (bind _output_get (Variables|Default|SetColorDMI _returnvalue))
  (Rendering|Material|SetVectorParameterValue _output_get "Color" (Variables|Default|GetPickupColor) :!class /Script/Engine.MaterialInstanceDynamic))

(fn UpdateDoorAngle
  (params (self2 :type Actor%20Object%20Reference))
  (return (select (> (Math|Vector|DotProduct (Math|Vector|GetUnitDirection(Vector) (Transformation|GetActorLocation) (Transformation|GetActorLocation self2)) (Transformation|GetActorForwardVector)) 0.0) 9e+01 -9e+01)))